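; Example pawn that starts an XD event flow and displays a live debug readout of the flows underway.
; BeginPlay activates Example_EventFlowGraphBlueprint through XDEventFlowManager.
; Each Tick, GetDesc walks the underway flows, their current sequences and those sequences' elements in nested loops.
; It builds one string from their debug names and dash markers, which is written to the TextRender component.
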(event EventBeginPlay
  (Class|XDEventFlowManager|ActiveEventFlow (Variables|Default|GetXD_EventFlowManager) "/XD_EventFlowSystem/Blueprints/Example_EventFlowGraphBlueprint.Example_EventFlowGraphBlueprint_C"))

(event Collision|EventActorBeginOverlap
  (params (OtherActor :type Actor%20Object%20Reference)))

(event EventTick
  (params (DeltaSeconds :type Float%20%28single-precision%29))
  (bind _desc1 (CallFunction|GetDesc (Variables|/Script/XD_EventFlowSystem.XD_EventFlowManager|GetUnderwayEventFlowList (Variables|Default|GetXD_EventFlowManager))))
  (Rendering|Components|TextRender|SetText (Variables|Default|GetTextRender) (Utilities|Text|ToText(String) _desc1)))

(fn ConstructionScript)

(fn GetDesc
  (params (Array :type Array%20of%20XD%20Event%20Flow%20Base%20Object%20References))
  (for _array_element Array
    (LocalVariables|SetDesc (Utilities|String|Append (LocalVariables|GetDesc) (Class|XDDebugFunctionLibrary|GetDebugName _array_element) " 
"))
    (for _array_element_2 (Variables|/Script/XD_EventFlowSystem.XD_EventFlowBase|GetCurrentEventFlowSequenceList _array_element)
      (LocalVariables|SetDesc (Utilities|String|Append "--" (LocalVariables|GetDesc) (Class|XDDebugFunctionLibrary|GetDebugName _array_element_2) " 
"))
      (for _array_element_3 (Variables|/Script/XD_EventFlowSystem.XD_EventFlowSequenceBase|GetEventFlowElementList _array_element_2)
        (LocalVariables|SetDesc (Utilities|String|Append "----" (LocalVariables|GetDesc) (Class|XDDebugFunctionLibrary|GetDebugName _array_element_3) " 
")))))
  (return (LocalVariables|GetDesc)))